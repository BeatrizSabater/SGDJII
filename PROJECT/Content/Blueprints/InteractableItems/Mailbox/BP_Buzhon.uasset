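; BP_Buzhon is an interactable mailbox that opens a quest list UI when the player interacts with it.
; Its box overlap registers or clears itself as the character's interactable actor.
; StartInteraction disables player input, clears the HUD's new-quest notice, and lazily creates or re-shows a cached W_MailboxTest widget in UI-only mode, refreshing its quests.
; The widget's close event collapses it and restores game input.
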(event OnComponentBeginOverlap(Box)
  (params (OverlappedComponent :type Primitive%20Component%20Object%20Reference) (OtherActor :type Actor%20Object%20Reference) (OtherComp :type Primitive%20Component%20Object%20Reference) (OtherBodyIndex :type Integer) (bFromSweep :type Boolean) (SweepResult :type Hit%20Result%20Structure%20%28by%20ref%29))
  ;[1 0 0.7969] Collision Box
  (bind _asthird_person_character (Utilities|Casting|CastToThirdPersonCharacter OtherActor))
  (Default|RegisterInteractableActor _asthird_person_character self))

(event OnComponentEndOverlap(Box)
  (params (OverlappedComponent :type Primitive%20Component%20Object%20Reference) (OtherActor :type Actor%20Object%20Reference) (OtherComp :type Primitive%20Component%20Object%20Reference) (OtherBodyIndex :type Integer))
  ;[1 0 0.7969] Collision Box
  (bind _asthird_person_character (Utilities|Casting|CastToThirdPersonCharacter OtherActor))
  (Default|RegisterInteractableActor _asthird_person_character))

(event Custom|CloseWidget
  (bind _returnvalue (Game|GetPlayerController 0))
  ;[0 1 0.7656] Close Widget
  (Widget|SetVisibility (Variables|Default|GetMailboxWidget) "Collapsed")
  (Variables|/Script/Engine.PlayerController|SetbShowMouseCursor _returnvalue false)
  (Input|SetInputModeGameOnly _returnvalue)
  (Input|EnableInput (.AsThird%20Person%20Character (Utilities|Casting|CastToThirdPersonCharacter (Game|Player|GetPlayerPawn 0))) _returnvalue))

(event EventStartInteraction
  (params (InteractiveActor :type Actor%20Object%20Reference))
  (bind _returnvalue (Game|GetPlayerController 0))
  (bind _asthird_person_character (Utilities|Casting|CastToThirdPersonCharacter InteractiveActor))
  ;[0.2656 0 1] Start Interaction (Interface Implementation)
  (Input|DisableInput _asthird_person_character (Game|GetPlayerController 0))
  (Default|NoNewQuestAvaible (Variables|/Game/Blueprints/Core/ThirdPersonCharacter.ThirdPersonCharacter_C|GetMainHUD _asthird_person_character))
  (Utilities|IsValid (Variables|Default|GetMailboxWidget)
    (:Is%20Valid
      (Widget|SetVisibility (Variables|Default|GetMailboxWidget) "Visible"))
    (:Is%20Not%20Valid
      (bind _returnvalue_2 (UserInterface|CreateWidget "/Game/Blueprints/InteractableItems/Mailbox/W_MailboxTest.W_MailboxTest_C"))
      (bind _output_get (Variables|Default|SetMailboxWidget _returnvalue_2))
      (UserInterface|Viewport|AddtoViewport _output_get 0)
      (EventDispatchers|BindEventtoCloseClicked _output_get (delegate Custom|CloseWidget))))
  (Variables|/Script/Engine.PlayerController|SetbShowMouseCursor _returnvalue true)
  (Input|SetInputModeUIOnly _returnvalue (Variables|Default|GetMailboxWidget) "LockInFullscreen")
  (Default|RefreshQuestList (Variables|Default|GetMailboxWidget)))

(fn ConstructionScript)