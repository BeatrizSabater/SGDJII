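; BP_HouseDoor is an interactable house door that teleports the player character to a fixed, hardcoded location.
; Its box overlap registers the door with the ThirdPersonCharacter as the current interactable and clears it on exit.
; StartInteraction disables input and fades the camera and audio out, sets a new boom length, boom rotation and FOV, teleports, then fades in and restores input, sequenced by delays.
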(event OnComponentBeginOverlap(Box)
  (params (OverlappedComponent :type Primitive%20Component%20Object%20Reference) (OtherActor :type Actor%20Object%20Reference) (OtherComp :type Primitive%20Component%20Object%20Reference) (OtherBodyIndex :type Integer) (bFromSweep :type Boolean) (SweepResult :type Hit%20Result%20Structure%20%28by%20ref%29))
  ;[0 0.7422 1] Collision Box
  (bind _asthird_person_character (Utilities|Casting|CastToThirdPersonCharacter OtherActor))
  (Default|RegisterInteractableActor _asthird_person_character self))

(event OnComponentEndOverlap(Box)
  (params (OverlappedComponent :type Primitive%20Component%20Object%20Reference) (OtherActor :type Actor%20Object%20Reference) (OtherComp :type Primitive%20Component%20Object%20Reference) (OtherBodyIndex :type Integer))
  ;[0 0.7422 1] Collision Box
  (bind _asthird_person_character (Utilities|Casting|CastToThirdPersonCharacter OtherActor))
  (Default|RegisterInteractableActor _asthird_person_character))

(event EventBeginPlay)

(event Collision|EventActorBeginOverlap
  (params (OtherActor :type Actor%20Object%20Reference)))

(event EventTick
  (params (DeltaSeconds :type Float%20%28single-precision%29)))

(event EventStartInteraction
  (params (InteractiveActor :type Actor%20Object%20Reference))
  (bind _returnvalue (Game|Player|GetPlayerPawn 0))
  (bind _asthird_person_character (Utilities|Casting|CastToThirdPersonCharacter _returnvalue))
  (bind _cameraboom (Variables|/Game/ThirdPersonBP/Blueprints/ThirdPersonCharacter.ThirdPersonCharacter_C|GetCameraBoom _asthird_person_character))
  (CameraFades|StartCameraFade :self (Game|GetPlayerCameraManager 0) :FromAlpha 0.7 :ToAlpha 1.0 :Duration 1.0 :bShouldFadeAudio true)
  (Input|DisableInput (Game|Player|GetPlayerPawn 0) (Game|GetPlayerController 0))
  (Utilities|FlowControl|Delay 0.9)
  (Variables|/Script/Engine.SpringArmComponent|SetTargetArmLength _cameraboom 2323.242676)
  (Variables|/Script/Engine.CameraComponent|SetFieldOfView (Variables|/Game/ThirdPersonBP/Blueprints/ThirdPersonCharacter.ThirdPersonCharacter_C|GetFollowCamera _asthird_person_character) 56.4286)
  (Transformation|SetRelativeRotation _cameraboom "-39.999817,-40.000160, 0" false false)
  (Transformation|SetActorLocationAndRotation (.AsThird%20Person%20Character (Utilities|Casting|CastToThirdPersonCharacter (Game|Player|GetPlayerPawn 0))) "-894.773560,5652.913574,-2766.334961" "0, 0, 0" false true)
  (CameraFades|StartCameraFade :self (Game|GetPlayerCameraManager 0) :FromAlpha 1.0 :Duration 1.0 :bShouldFadeAudio true)
  (Utilities|FlowControl|Delay 0.98)
  (Input|EnableInput (Game|Player|GetPlayerPawn 0) (Game|GetPlayerController 0)))

(fn ConstructionScript)