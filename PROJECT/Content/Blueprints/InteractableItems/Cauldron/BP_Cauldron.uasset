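; Interactable cauldron for brewing potions, cycling through idle, brewing and ready states, with an outline and interaction registration on player overlap.
; Interacting opens the synthesizer widget, whose combination result starts a timeline-driven progress bar timed by recipe and cauldron upgrade.
; Failed mixes yield an erroneous potion and call a random-ingredient unlock.
; Closing the result popup puts the item in the inventory and handles recipe unlocks and potion visibility.
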(event OnComponentBeginOverlap(Box)
  (params (OverlappedComponent :type Primitive%20Component%20Object%20Reference) (OtherActor :type Actor%20Object%20Reference) (OtherComp :type Primitive%20Component%20Object%20Reference) (OtherBodyIndex :type Integer) (bFromSweep :type Boolean) (SweepResult :type Hit%20Result%20Structure%20%28by%20ref%29))
  ;[0 0.7422 1] Collision Box
  (bind _asthird_person_character (Utilities|Casting|CastToThirdPersonCharacter OtherActor))
  (CallFunction|CreateOutline)
  (Default|RegisterInteractableActor _asthird_person_character self))

(event OnComponentEndOverlap(Box)
  (params (OverlappedComponent :type Primitive%20Component%20Object%20Reference) (OtherActor :type Actor%20Object%20Reference) (OtherComp :type Primitive%20Component%20Object%20Reference) (OtherBodyIndex :type Integer))
  ;[0 0.7422 1] Collision Box
  (bind _asthird_person_character (Utilities|Casting|CastToThirdPersonCharacter OtherActor))
  (Default|RegisterInteractableActor _asthird_person_character)
  (CallFunction|DeleteOutline))

(event Custom|CreateOutline
  ;[1 0.4922 0] OutLine
  (if (not (Variables|Default|GetbThereIsOutline))
    (bind _returnvalue (AddComponent|AddStaticMeshComponent true (Transformation|GetWorldTransform (Variables|Default|GetMesh))))
    (bind _output_get (Variables|Default|SetOutlinerMesh _returnvalue))
    (Components|StaticMesh|SetStaticMesh _output_get (Variables|/Script/Engine.StaticMeshComponent|GetStaticMesh (Variables|Default|GetMesh)))
    (bind _returnvalue_2 (Rendering|Material|CreateDynamicMaterialInstance _output_get 0 "/Game/Materials/Outline/m_outline_Inst.m_outline_Inst" "None" :!class /Script/Engine.PrimitiveComponent))
    (Rendering|Material|SetVectorParameterValue _returnvalue_2 "color" "(R=0.901042,G=0.671726,B=0.110566,A=1.000000)" :!class /Script/Engine.MaterialInstanceDynamic)
    (Rendering|Material|SetScalarParameterValue _returnvalue_2 "Scale" 2.0 :!class /Script/Engine.MaterialInstanceDynamic)
    (Variables|Default|SetbThereIsOutline true)))

(event Custom|DeleteOutline
  (bind _outlinermesh (Variables|Default|GetOutlinerMesh))
  ;[1 0.4922 0] OutLine
  (Utilities|IsValid _outlinermesh
    (:Is%20Valid
      (Components|DestroyComponent _outlinermesh)
      (Variables|Default|SetbThereIsOutline false))))

(event Custom|MakingPotion
  (params (Successful :type Boolean) (Recipe :type ST%20Recipes%20Struct%20Structure))
  (bind (_nombre _descripción _ingrediente1 _ingrediente2 _ingrediente3 _tiempo) (Utilities|Struct|BreakST_RecipesStruct Recipe))
  (bind _returnvalue (Game|GetPlayerCameraManager 0))
  (bind _returnvalue_2 (Game|GetPlayerCameraManager 0))
  (bind _widget (Variables|Default|GetWidget))
  (bind _widget_2 (Variables|Default|GetWidget))
  (Variables|Default|SetbSuccessful Successful)
  (Variables|Default|SetCauldronState "NewEnumerator1")
  (CallFunction|CloseCraftWidget)
  (Rendering|SetVisibility (Variables|Default|GetWidget) true true)
  (Components|Timeline|PlayfromStart (Variables|Default|GetTL_ProgressBar))
  (if Successful
    (bind _outrownames (DataTable|GetDataTableRowNames "/Game/Blueprints/Core/Datatables/Lista_de_ítems_-_Hoja_1.Lista_de_ítems_-_Hoja_1"))
    (bind _array_element (Utilities|Array|ForEachLoopwithBreak _outrownames :!label _label)
      (:LoopBody
        (bind _returnvalue_3 (Utilities|GetDataTableRow "/Game/Blueprints/Core/Datatables/Lista_de_ítems_-_Hoja_1.Lista_de_ítems_-_Hoja_1" _array_element)
          (:then
            (if (Utilities|Enum|Equal(Enum) (.Nombre (Utilities|Struct|BreakST_ItemStruct _returnvalue_3)) _nombre)
              (Variables|Default|SetCreatedNewItem (Utilities|Struct|MakeST_ItemSave _returnvalue_3 false))
              (goto _label Break)))))
      (:Completed
        (Components|Timeline|SetPlayRate (Variables|Default|GetTL_ProgressBar) (/ 1e+02 (- _tiempo (Math|Conversions|ToFloat(Integer) (Variables|/Game/Blueprints/Core/GI_MainGameInstance.GI_MainGameInstance_C|GetCauldronUpgrade (.AsGI%20Main%20Game%20Instance (Utilities|Casting|CastToGI_MainGameInstance (Game|GetGameInstance))))))))
        (Utilities|IsValid _returnvalue_2
          (:Is%20Valid
            (Transformation|SetRelativeRotation _widget_2 (Math|Rotator|MakeRotator 0.0 0.0 (+ (.yaw (Math|Rotator|FindLookatRotation (Transformation|GetWorldLocation _widget_2) (Camera|GetCameraLocation _returnvalue_2))) 2.7e+02)) false false)))))
    (else
      (bind _returnvalue_4 (Utilities|GetDataTableRow "/Game/Blueprints/Core/Datatables/Lista_de_ítems_-_Hoja_1.Lista_de_ítems_-_Hoja_1" "PocionErrónea")
        (:then
          (Variables|Default|SetCreatedNewItem (Utilities|Struct|MakeST_ItemSave _returnvalue_4 false))
          (bind _successful (CallFunction|UnlockRandomIngredient))
          (Variables|Default|SetbIsIngredientUnlocked _successful)
          (Components|Timeline|SetPlayRate (Variables|Default|GetTL_ProgressBar) (/ 1e+02 1.0))
          (Utilities|IsValid _returnvalue
            (:Is%20Valid
              (Transformation|SetRelativeRotation _widget (Math|Rotator|MakeRotator 0.0 0.0 (+ (.yaw (Math|Rotator|FindLookatRotation (Transformation|GetWorldLocation _widget) (Camera|GetCameraLocation _returnvalue))) 2.7e+02)) false false))))))))

(event Custom|CloseCraftWidget
  (bind _returnvalue (Game|GetPlayerController 0))
  (bind _craftwidget (Variables|Default|GetCraftWidget))
  (bind _ingrediente01 (Variables|/Game/Blueprints/InteractableItems/Cauldron/W_Synthesizer.W_Synthesizer_C|GetIngrediente01 _craftwidget))
  (bind _ingrediente02 (Variables|/Game/Blueprints/InteractableItems/Cauldron/W_Synthesizer.W_Synthesizer_C|GetIngrediente02 _craftwidget))
  (bind _ingrediente03 (Variables|/Game/Blueprints/InteractableItems/Cauldron/W_Synthesizer.W_Synthesizer_C|GetIngrediente03 _craftwidget))
  (Variables|/Game/UI/W_DragTo.W_DragTo_C|Setitem _ingrediente01 "")
  (Default|RefreshSlot _ingrediente01)
  (Default|EnableDragto _ingrediente01)
  (Variables|/Game/UI/W_DragTo.W_DragTo_C|Setitem _ingrediente02 "")
  (Default|DisableDragto _ingrediente02)
  (Default|RefreshSlot _ingrediente02)
  (Variables|/Game/UI/W_DragTo.W_DragTo_C|Setitem _ingrediente03 "")
  (Default|DisableDragto _ingrediente03)
  (Default|RefreshSlot _ingrediente03)
  (Widget|SetVisibility _craftwidget "Collapsed")
  (Input|SetInputModeGameOnly _returnvalue)
  (Input|EnableInput _returnvalue _returnvalue)
  (Variables|/Script/Engine.PlayerController|SetbShowMouseCursor _returnvalue false))

(event Custom|CloseTab
  (bind _returnvalue (Game|GetGameInstance))
  (bind _returnvalue_2 (Game|GetPlayerController 0))
  (bind _asgi_main_game_instance (Utilities|Casting|CastToGI_MainGameInstance _returnvalue))
  (bind _inventoryarray (Variables|/Game/Blueprints/Core/GI_MainGameInstance.GI_MainGameInstance_C|GetInventoryArray _asgi_main_game_instance))
  (Input|SetInputModeGameOnly (Game|GetPlayerController 0))
  (Widget|SetVisibility (Variables|Default|GetPopUpWidget) "Collapsed")
  (bind (_array_element _array_index) (Utilities|Array|ForEachLoopwithBreak _inventoryarray :!label _label)
    (:LoopBody
      (if (Utilities|Array|IsEmpty (.Nombre (Utilities|Struct|BreakST_ItemStruct (.ItemInfo (Utilities|Struct|BreakST_ItemSave _array_element)))))
        (bind _isalreadyunlocked (CallFunction|UnlockRecipebyName (.nombre (.ItemInfo (Utilities|Struct|BreakST_ItemSave (Variables|Default|GetCreatedNewItem))))))
        (if _isalreadyunlocked
          (Utilities|Array|SetArrayElem _inventoryarray _array_index (Variables|Default|GetCreatedNewItem))
          (Variables|Default|SetCreatedNewItem "")
          (Variables|Default|SetbSuccessful false)
          (goto _label Break)
          (else
            (bind _outactors (Actor|GetAllActorsOfClass "/Game/Blueprints/InteractableItems/Cauldron/BP_Potion.BP_Potion_C"))
            (bind _array_element_2 (Utilities|Array|ForEachLoopwithBreak _outactors :!label _label_2)
              (:LoopBody
                (if (Utilities|Enum|Equal(Enum) (Variables|/Game/Blueprints/InteractableItems/Cauldron/BP_Potion.BP_Potion_C|GetName _array_element_2) (.nombre (.ItemInfo (Utilities|Struct|BreakST_ItemSave (Variables|Default|GetCreatedNewItem)))))
                  (Rendering|SetVisibility (Variables|/Game/Blueprints/InteractableItems/Cauldron/BP_Potion.BP_Potion_C|GetStaticMesh _array_element_2) true true)
                  (goto _label_2 Break)))
              (:Completed
                (Utilities|Array|SetArrayElem _inventoryarray _array_index (Variables|Default|GetCreatedNewItem))
                (Variables|Default|SetCreatedNewItem "")
                (Variables|Default|SetbSuccessful false)
                (goto _label Break)))))))
    (:Completed
      (if (Utilities|Array|IsEmpty (.nombre (.ItemInfo (Utilities|Struct|BreakST_ItemSave (Variables|Default|GetCreatedNewItem)))))
        (Variables|Default|SetCauldronState "NewEnumerator0")
        (Rendering|SetVisibility (Variables|Default|GetPlane) false true))
      (Input|SetInputModeGameOnly _returnvalue_2)
      (Input|EnableInput _returnvalue_2 _returnvalue_2)
      (Variables|/Script/Engine.PlayerController|SetbShowMouseCursor _returnvalue_2 false))))

(event Collision|EventActorBeginOverlap
  (params (OtherActor :type Actor%20Object%20Reference)))

(event EventStartInteraction
  (params (InteractiveActor :type Actor%20Object%20Reference))
  (bind _returnvalue (Game|GetPlayerController 0))
  (bind _returnvalue_2 (Game|GetPlayerController 0))
  (bind _cauldronstate (Variables|Default|GetCauldronState))
  (if (Utilities|Enum|NotEqual(Enum) _cauldronstate "NewEnumerator1")
    (if (Utilities|Enum|Equal(Enum) _cauldronstate "NewEnumerator0")
      (Variables|Default|SetbSuccessful false)
      (Variables|Default|SetCreatedNewItem "")
      (Input|DisableInput (.AsThird%20Person%20Character (Utilities|Casting|CastToThirdPersonCharacter InteractiveActor)) (Game|GetPlayerController 0))
      (Utilities|IsValid (Variables|Default|GetCraftWidget)
        (:Is%20Valid
          (Widget|SetVisibility (Variables|Default|GetCraftWidget) "Visible"))
        (:Is%20Not%20Valid
          (bind _returnvalue_3 (UserInterface|CreateWidget "/Game/Blueprints/InteractableItems/Cauldron/W_Synthesizer.W_Synthesizer_C"))
          (bind _output_get (Variables|Default|SetCraftWidget _returnvalue_3))
          (UserInterface|Viewport|AddtoViewport _output_get 0)
          (EventDispatchers|BindEventtoWidgetClosed _output_get (delegate Custom|CloseCraftWidget))
          (EventDispatchers|BindEventtoMadeCombination _output_get (delegate Custom|MakingPotion))))
      (Variables|/Script/Engine.PlayerController|SetbShowMouseCursor _returnvalue true)
      (Input|SetInputModeUIOnly _returnvalue (Variables|Default|GetCraftWidget) "LockInFullscreen")
      (Default|RefreshInventory (Variables|Default|GetCraftWidget))
      (else
        (Input|DisableInput (.AsThird%20Person%20Character (Utilities|Casting|CastToThirdPersonCharacter InteractiveActor)) (Game|GetPlayerController 0))
        (Utilities|IsValid (Variables|Default|GetPopUpWidget)
          (:Is%20Valid
            (Widget|SetVisibility (Variables|Default|GetPopUpWidget) "Visible"))
          (:Is%20Not%20Valid
            (bind _returnvalue_4 (UserInterface|CreateWidget "/Game/Blueprints/InteractableItems/Cauldron/W_CombinationResult.W_CombinationResult_C" 0 (Variables|Default|GetbSuccessful) (Variables|Default|GetbIsIngredientUnlocked)))
            (bind _output_get_2 (Variables|Default|SetPopUpWidget _returnvalue_4))
            (UserInterface|Viewport|AddtoViewport _output_get_2 0)
            (EventDispatchers|BindEventtoWidgetClose _returnvalue_4 (delegate Custom|CloseTab))))
        (Variables|/Script/Engine.PlayerController|SetbShowMouseCursor _returnvalue_2 true)
        (Input|SetInputModeGameandUI _returnvalue_2 (Variables|Default|GetPopUpWidget) "LockInFullscreen" true)
        (Default|RefreshItem (Variables|Default|GetPopUpWidget) (.ItemInfo (Utilities|Struct|BreakST_ItemSave (Variables|Default|GetCreatedNewItem))) (Variables|Default|GetbSuccessful) (Variables|Default|GetbIsIngredientUnlocked))))))

(fn ConstructionScript)