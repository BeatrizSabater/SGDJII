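; Main game instance that sets up recipe, quest and inventory state on Init.
; It loads the save into SaveGameData, or without one spawns BP_Recipe actors from the combinations table into Gremory and pre-unlocks one recipe.
; It also fills empty Quests with BP_Quest actors from the missions table and places a "Calabaza" BP_Item in Inventory.
; Loaded data is only stored, and the save-creation nodes are unconnected.
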(event EventInit
  (bind _gremory (Variables|Default|GetGremory))
  (bind _output (Utilities|Array|Get(acopy) _gremory 22))
  (Utilities|FlowControl|Sequence
    (:then_0
      (bind _returnvalue (SaveGame|DoesSaveGameExist (Variables|Default|GetSaveSlotName)))
      (if _returnvalue
        (bind _returnvalue_2 (SaveGame|LoadGamefromSlot (Variables|Default|GetSaveSlotName)))
        (bind _assg_main_saved_game (Utilities|Casting|CastToSG_MainSavedGame _returnvalue_2))
        (Variables|Default|SetSaveGameData _assg_main_saved_game)
        (else
          (bind _outrownames (DataTable|GetDataTableRowNames "/Game/Test/InventoryTest/Lista_de_Combinaciones_-_Hoja_1.Lista_de_Combinaciones_-_Hoja_1"))
          (bind _array_element (Utilities|Array|ForEachLoopwithBreak _outrownames)
            (:LoopBody
              (bind _returnvalue_3 (Utilities|GetDataTableRow "/Game/Test/InventoryTest/Lista_de_Combinaciones_-_Hoja_1.Lista_de_Combinaciones_-_Hoja_1" _array_element)
                (:then
                  (bind _returnvalue_4 (Game|SpawnActorfromClass "/Game/Test/InventoryTest/BP_Recipe.BP_Recipe_C" (Math|Transform|MakeTransform "0, 0, 0" "0, 0, 0" "1,1,1") "AlwaysSpawn" 0 _returnvalue_3 0))
                  (Utilities|Array|Add (Variables|Default|GetGremory) _returnvalue_4))))
            (:Completed
              (Variables|/Game/Test/InventoryTest/BP_Recipe.BP_Recipe_C|SetbUnlocked _output true)
              (Variables|/Game/Test/InventoryTest/BP_Recipe.BP_Recipe_C|SetbDiscovered _output (Utilities|Array|MakeArray false true)))))))
    (:then_1
      (if (== (Utilities|Array|Length (Variables|Default|GetQuests)) 0)
        (bind _outrownames_2 (DataTable|GetDataTableRowNames "/Game/Test/QuestsTest/Lista_de_misiones_y_recompensas_-_Hoja_1.Lista_de_misiones_y_recompensas_-_Hoja_1"))
        (for _array_element_2 _outrownames_2
          (bind _returnvalue_5 (Utilities|GetDataTableRow "/Game/Test/QuestsTest/Lista_de_misiones_y_recompensas_-_Hoja_1.Lista_de_misiones_y_recompensas_-_Hoja_1" _array_element_2)
            (:then
              (bind _returnvalue_6 (Game|SpawnActorfromClass "/Game/Test/QuestsTest/BP_Quest.BP_Quest_C" (Math|Transform|MakeTransform "0, 0, 0" "0, 0, 0" "1,1,1") "AlwaysSpawn" 0 _returnvalue_5 0))
              (Utilities|Array|Add (Variables|Default|GetQuests) _returnvalue_6))))))
    (:then_2
      (bind _returnvalue_7 (Utilities|GetDataTableRow "/Game/Test/InventoryTest/Lista_de_ítems_-_Hoja_1.Lista_de_ítems_-_Hoja_1" "Calabaza")
        (:then
          (bind _returnvalue_8 (Game|SpawnActorfromClass "/Game/Test/InventoryTest/BP_Item.BP_Item_C" (Math|Transform|MakeTransform "0, 0, 0" "0.000000, 0, 0" "1,1,1") "AlwaysSpawn" 0 _returnvalue_7 0))
          (Utilities|Array|SetArrayElem (Variables|Default|GetInventory) 0 _returnvalue_8))))))