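; Blueprint function library of shared helpers for items, inventory, quests, recipes and upgrades.
; Loops over DataTables to find items by name, and over GI_MainGameInstance arrays to fill or count empty slots and update saved states.
; Recipe unlocks decrement a counter that, at zero, resets and triggers UnlockNextQuest with a HUD notice; upgrade names set chest and cauldron variables.
; GetQuestByTitle is unfinished: its title comparison is unconnected and it returns no row.
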(fn FindItemDatatable
  (params (Name :type String))
  (bind _outrownames (DataTable|GetDataTableRowNames "/Game/Blueprints/Core/Datatables/Lista_de_ítems_-_Hoja_1.Lista_de_ítems_-_Hoja_1"))
  (for _array_element _outrownames
    (bind _returnvalue (Utilities|GetDataTableRow "/Game/Blueprints/Core/Datatables/Lista_de_ítems_-_Hoja_1.Lista_de_ítems_-_Hoja_1" _array_element)
      (:then
        (if (Utilities|Enum|Equal(Enum) Name (.Nombre (Utilities|Struct|BreakST_ItemStruct _returnvalue)))
          (return _returnvalue)))))
  (return ""))

(fn AddItemtoInventory
  (params (ST_ItemStruct :type ST%20Item%20Struct%20Structure%20%28by%20ref%29))
  (bind _returnvalue (Game|GetGameInstance))
  (bind _asgi_main_game_instance (Utilities|Casting|CastToGI_MainGameInstance _returnvalue))
  (bind _newinventory (Variables|/Game/Blueprints/Core/GI_MainGameInstance.GI_MainGameInstance_C|GetNewInventory _asgi_main_game_instance))
  (for (_array_element _array_index) _newinventory
    (if (Utilities|Array|IsEmpty (.Nombre (Utilities|Struct|BreakST_ItemStruct (.ItemInfo (Utilities|Struct|BreakST_ItemSave _array_element)))))
      (Utilities|Array|SetArrayElem _newinventory _array_index (Utilities|Struct|MakeST_ItemSave ST_ItemStruct false))
      (return true)))
  (return false))

(fn GetQuestbyTitle
  (params (Title :type Text))
  (bind _outrownames (DataTable|GetDataTableRowNames "/Game/Blueprints/Core/Datatables/Lista_de_misiones_y_recompensas_-_Hoja_1.Lista_de_misiones_y_recompensas_-_Hoja_1"))
  (for _array_element _outrownames
    (bind _returnvalue (Utilities|GetDataTableRow "/Game/Blueprints/Core/Datatables/Lista_de_misiones_y_recompensas_-_Hoja_1.Lista_de_misiones_y_recompensas_-_Hoja_1" _array_element)
      (:then
        (if (Utilities|Enum|Equal(Enum) "" "")
          (return ""))))))

(fn ChangeQuestState
  (params (NewQuestState :type E_QuestState%20Enum :default "NewEnumerator0") (QuestTitle :type Text) (Completed :type Boolean))
  (bind _returnvalue (Game|GetGameInstance))
  (bind _asgi_main_game_instance (Utilities|Casting|CastToGI_MainGameInstance _returnvalue))
  (bind _newquests (Variables|/Game/Blueprints/Core/GI_MainGameInstance.GI_MainGameInstance_C|GetNewQuests _asgi_main_game_instance))
  (for (_array_element _array_index) _newquests
    (if (Utilities|Enum|Equal(Enum) (.Título (Utilities|Struct|BreakST_QuestStruct (.QuestStruct (Utilities|Struct|BreakST_QuestSave _array_element)))) QuestTitle)
      (Utilities|Array|SetArrayElem _newquests _array_index (Utilities|Struct|MakeST_QuestSave NewQuestState (.QuestStruct (Utilities|Struct|BreakST_QuestSave _array_element)) Completed)))))

(fn GetAvaibleInventorySlots
  (for _array_element (Variables|/Game/Blueprints/Core/GI_MainGameInstance.GI_MainGameInstance_C|GetNewInventory (.AsGI%20Main%20Game%20Instance (Utilities|Casting|CastToGI_MainGameInstance (Game|GetGameInstance))))
    (if (Utilities|Array|IsEmpty (.nombre (.ItemInfo (Utilities|Struct|BreakST_ItemSave _array_element))))
      (Math|Integer|IncrementInt (LocalVariables|GetNumInventorySlots))))
  (return (LocalVariables|GetNumInventorySlots)))

(fn UnlockNextQuest
  (for _array_element (Variables|/Game/Blueprints/Core/GI_MainGameInstance.GI_MainGameInstance_C|GetNewQuests (.AsGI%20Main%20Game%20Instance (Utilities|Casting|CastToGI_MainGameInstance (Game|GetGameInstance))))
    (if (Utilities|Enum|Equal(Enum) (.QuestState (Utilities|Struct|BreakST_QuestSave _array_element)) "NewEnumerator4")
      (CallFunction|ChangeQuestState "NewEnumerator0" (.Título (Utilities|Struct|BreakST_QuestStruct (.QuestStruct (Utilities|Struct|BreakST_QuestSave _array_element)))) false)
      (Default|NewQuestAvaible (Variables|/Game/ThirdPersonBP/Blueprints/ThirdPersonCharacter.ThirdPersonCharacter_C|GetMainHUD (.AsThird%20Person%20Character (Utilities|Casting|CastToThirdPersonCharacter (Game|Player|GetPlayerPawn 0)))))
      (return)))
  ;[0.6875 1 0] Aqui podrian ir las misiones repetidas
  (return))

(fn UnlockRecipebyName
  (params (Name :type String))
  (bind _returnvalue (Game|GetGameInstance))
  (bind _returnvalue_2 (Game|GetGameInstance))
  (bind _asgi_main_game_instance (Utilities|Casting|CastToGI_MainGameInstance _returnvalue))
  (bind _asgi_main_game_instance_2 (Utilities|Casting|CastToGI_MainGameInstance _returnvalue_2))
  (bind _newgremory (Variables|/Game/Blueprints/Core/GI_MainGameInstance.GI_MainGameInstance_C|GetNewGremory _asgi_main_game_instance_2))
  (for (_array_element _array_index) _newgremory
    (if (Utilities|Enum|Equal(Enum) Name (.Nombre (Utilities|Struct|BreakST_RecipesStruct (.Recipe (Utilities|Struct|BreakST_RecipeSave _array_element)))))
      (if (not (.Unlocked (Utilities|Struct|BreakST_RecipeSave _array_element)))
        (Utilities|Array|SetArrayElem _newgremory _array_index (Utilities|Struct|MakeST_RecipeSave (.Recipe (Utilities|Struct|BreakST_RecipeSave _array_element)) true (.Dicovered (Utilities|Struct|BreakST_RecipeSave _array_element))))
        (bind _result (Math|Integer|DecrementInt (Variables|/Game/Blueprints/Core/GI_MainGameInstance.GI_MainGameInstance_C|GetCombinationsLeftForNewQuest _asgi_main_game_instance))
          (:%20%20
            (if (== _result 0)
              (Variables|/Game/Blueprints/Core/GI_MainGameInstance.GI_MainGameInstance_C|SetCombinationsLeftForNewQuest _asgi_main_game_instance 3)
              (CallFunction|UnlockNextQuest)
              (return false)))))))
  (return false))

(fn UnlockUpgrade
  (params (UpgradeName :type String))
  (bind _returnvalue (Game|GetGameInstance))
  (bind _returnvalue_2 (Game|GetGameInstance))
  (bind _asgi_main_game_instance (Utilities|Casting|CastToGI_MainGameInstance _returnvalue))
  (bind _asgi_main_game_instance_2 (Utilities|Casting|CastToGI_MainGameInstance _returnvalue_2))
  (switch string UpgradeName
    (:Baúl
      (Variables|/Game/Blueprints/Core/GI_MainGameInstance.GI_MainGameInstance_C|SetChestUnlocked _asgi_main_game_instance true))
    (:Mejora%20de%20caldero%20I
      (Variables|/Game/Blueprints/Core/GI_MainGameInstance.GI_MainGameInstance_C|SetCauldronUpgrade _asgi_main_game_instance 10))
    (:Caldero%20I
      (Variables|/Game/Blueprints/Core/GI_MainGameInstance.GI_MainGameInstance_C|SetCauldronIUnlocked _asgi_main_game_instance true))
    (:Mejora%20de%20caldero%20II
      (Variables|/Game/Blueprints/Core/GI_MainGameInstance.GI_MainGameInstance_C|SetCauldronUpgrade _asgi_main_game_instance_2 15))
    (:Caldero%20II
      (Variables|/Game/Blueprints/Core/GI_MainGameInstance.GI_MainGameInstance_C|SetCauldronIIUnlocked _asgi_main_game_instance_2 false))
    (:Mejora%20caldero%20III
      (Variables|/Game/Blueprints/Core/GI_MainGameInstance.GI_MainGameInstance_C|SetCauldronUpgrade _asgi_main_game_instance_2 20))))