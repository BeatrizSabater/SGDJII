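; Interactable extraction point where the player extracts a data-table-defined item into their inventory.
; Sphere overlap registers it with the character, and RefreshData sets whether it is enabled and which item it yields.
; Interaction runs a state enum: it locks movement, checks inventory space, shows HUD progress during a timed delay, then adds the item.
; When the remaining-extraction counter hits zero, it enters a timed depleted state before returning to idle, without resetting the counter.
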(event OnComponentEndOverlap(Sphere)
  (params (OverlappedComponent :type Primitive%20Component%20Object%20Reference) (OtherActor :type Actor%20Object%20Reference) (OtherComp :type Primitive%20Component%20Object%20Reference) (OtherBodyIndex :type Integer))
  ;[0 0.7422 1] Collision Box
  (if (Variables|Default|GetbEnabled)
    (bind _asthird_person_character (Utilities|Casting|CastToThirdPersonCharacter OtherActor))
    (Default|RegisterInteractableActor _asthird_person_character)))

(event OnComponentBeginOverlap(Sphere)
  (params (OverlappedComponent :type Primitive%20Component%20Object%20Reference) (OtherActor :type Actor%20Object%20Reference) (OtherComp :type Primitive%20Component%20Object%20Reference) (OtherBodyIndex :type Integer) (bFromSweep :type Boolean) (SweepResult :type Hit%20Result%20Structure%20%28by%20ref%29))
  ;[0 0.7422 1] Collision Box
  (if (Variables|Default|GetbEnabled)
    (bind _asthird_person_character (Utilities|Casting|CastToThirdPersonCharacter OtherActor))
    (Default|RegisterInteractableActor _asthird_person_character self)
    (if (Utilities|Enum|Equal(Enum) (Variables|Default|GetExtractionPointState) "NewEnumerator2")
      (Default|ShowExtactNotText (Variables|/Game/Blueprints/Core/ThirdPersonCharacter.ThirdPersonCharacter_C|GetMainHUD _asthird_person_character)))))

(event Custom|RefreshData
  (params (Enabled :type Boolean) (ExtactableItemDataTable :type Data%20Table%20Row%20Handle%20Structure))
  ;[0.1615 0.3514 1] Begin Play
  (Variables|Default|SetbEnabled Enabled)
  (Variables|Default|SetExtractableItemDataTable ExtactableItemDataTable)
  (if (Variables|Default|GetbEnabled)
    (bind _returnvalue (Utilities|GetDataTableRow (.DataTable (Utilities|Struct|BreakDataTableRowHandle (Variables|Default|GetExtractableItemDataTable))) (.RowName (Utilities|Struct|BreakDataTableRowHandle (Variables|Default|GetExtractableItemDataTable))))
      (:then
        (Variables|Default|SetExtractableItemInfo _returnvalue)))))

(event Custom|ProgressBar
  (bind _returnvalue (Game|Player|GetPlayerPawn 0))
  (bind _returnvalue_2 (Game|Player|GetPlayerPawn 0))
  (bind _asthird_person_character (Utilities|Casting|CastToThirdPersonCharacter _returnvalue_2))
  (bind _asthird_person_character_2 (Utilities|Casting|CastToThirdPersonCharacter _returnvalue))
  (bind _mainhud (Variables|/Game/Blueprints/Core/ThirdPersonCharacter.ThirdPersonCharacter_C|GetMainHUD _asthird_person_character))
  ;[0.7812 1 0] ProgressBar
  (bind _avaibleinventoryslots (CallFunction|GetAvailableInventorySlots))
  (if (not (== _avaibleinventoryslots 0))
    (Default|StartExtracting _mainhud)
    (Utilities|FlowControl|Delay 6.0)
    (Variables|/Game/Blueprints/Core/ThirdPersonCharacter.ThirdPersonCharacter_C|SetbCanMove (.AsThird%20Person%20Character (Utilities|Casting|CastToThirdPersonCharacter (Game|Player|GetPlayerPawn 0))) true)
    (bind _successful (CallFunction|AddItemtoInventory (Variables|Default|GetExtractableItemInfo)))
    (if _successful
      (Default|ItemPickedUp (Variables|/Game/Blueprints/Core/ThirdPersonCharacter.ThirdPersonCharacter_C|GetMainHUD (.AsThird%20Person%20Character (Utilities|Casting|CastToThirdPersonCharacter (Game|Player|GetPlayerPawn 0)))) (Variables|Default|GetExtractableItemInfo))
      (bind _result (Math|Integer|DecrementInt (Variables|Default|GetExtractionTimesLeft))
        (:%20%20
          (if (== _result 0)
            (Variables|Default|SetExtractionPointState "NewEnumerator2")
            (Default|ShowExtactNotText _mainhud)
            (Utilities|FlowControl|Delay 1.2e+02)
            (Variables|Default|SetExtractionPointState "NewEnumerator0")
            (else
              (Variables|Default|SetExtractionPointState "NewEnumerator0")))))
      (else
        (Variables|Default|SetExtractionPointState "NewEnumerator0")))
    (else
      (Variables|/Game/Blueprints/Core/ThirdPersonCharacter.ThirdPersonCharacter_C|SetbCanMove _asthird_person_character_2 true)
      (Default|InventoryFull (Variables|/Game/Blueprints/Core/ThirdPersonCharacter.ThirdPersonCharacter_C|GetMainHUD _asthird_person_character_2))
      (Variables|Default|SetExtractionPointState "NewEnumerator0"))))

(event EventStartInteraction
  (params (InteractiveActor :type Actor%20Object%20Reference))
  (bind _asthird_person_character (Utilities|Casting|CastToThirdPersonCharacter InteractiveActor))
  ;[1 0 0] Event Start Interaction
  (if (Variables|Default|GetbEnabled)
    (if (Utilities|Enum|Equal(Enum) (Variables|Default|GetExtractionPointState) "NewEnumerator0")
      (Variables|/Game/Blueprints/Core/ThirdPersonCharacter.ThirdPersonCharacter_C|SetbCanMove _asthird_person_character false)
      (Variables|Default|SetExtractionPointState "NewEnumerator1")
      (CallFunction|ProgressBar))
    (elif (Utilities|Enum|Equal(Enum) (Variables|Default|GetExtractionPointState) "NewEnumerator2")
      (Default|ShowExtactNotText (Variables|/Game/Blueprints/Core/ThirdPersonCharacter.ThirdPersonCharacter_C|GetMainHUD _asthird_person_character)))))

(fn ConstructionScript
  (Components|StaticMesh|SetStaticMesh (Variables|Default|GetMesh) (Variables|Default|GetStaticMesh))
  (Components|Sphere|SetSphereRadius (Variables|Default|GetSphere) (Variables|Default|GetSphereCollisionRadius) true))