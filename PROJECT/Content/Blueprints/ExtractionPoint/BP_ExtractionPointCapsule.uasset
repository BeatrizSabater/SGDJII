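; Interactable extraction point that gives the player an item from a data table row when the inventory has a free slot.
; Capsule overlap registers it with the character; interacting locks movement during a timed HUD progress before adding the item.
; Exhausting its extraction count starts a cooldown state, though the count is never reset.
; Construction applies mesh and capsule size; outline events add or destroy a duplicate mesh with a dynamic outline material.
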(event OnComponentBeginOverlap(Capsule)
  (params (OverlappedComponent :type Primitive%20Component%20Object%20Reference) (OtherActor :type Actor%20Object%20Reference) (OtherComp :type Primitive%20Component%20Object%20Reference) (OtherBodyIndex :type Integer) (bFromSweep :type Boolean) (SweepResult :type Hit%20Result%20Structure%20%28by%20ref%29))
  ;[0 0.7422 1] Collision Box
  (if (Variables|Default|GetbEnabled)
    (bind _asthird_person_character (Utilities|Casting|CastToThirdPersonCharacter OtherActor))
    (Default|RegisterInteractableActor _asthird_person_character self)
    (if (Utilities|Enum|Equal(Enum) (Variables|Default|GetExtractionPointState) "NewEnumerator2")
      (Default|ShowExtactNotText (Variables|/Game/Blueprints/Core/ThirdPersonCharacter.ThirdPersonCharacter_C|GetMainHUD _asthird_person_character)))))

(event OnComponentEndOverlap(Capsule)
  (params (OverlappedComponent :type Primitive%20Component%20Object%20Reference) (OtherActor :type Actor%20Object%20Reference) (OtherComp :type Primitive%20Component%20Object%20Reference) (OtherBodyIndex :type Integer))
  ;[0 0.7422 1] Collision Box
  (if (Variables|Default|GetbEnabled)
    (bind _asthird_person_character (Utilities|Casting|CastToThirdPersonCharacter OtherActor))
    (Default|RegisterInteractableActor _asthird_person_character)))

(event Custom|CreateOutline
  ;[1 0.4922 0] OutLine
  (if (not (Variables|Default|GetbThereIsOutline))
    (bind _returnvalue (AddComponent|AddStaticMeshComponent true (Transformation|GetWorldTransform (Variables|Default|GetMesh))))
    (bind _output_get (Variables|Default|SetOutlinerMesh _returnvalue))
    (Components|StaticMesh|SetStaticMesh _output_get (Variables|/Script/Engine.StaticMeshComponent|GetStaticMesh (Variables|Default|GetMesh)))
    (bind _returnvalue_2 (Rendering|Material|CreateDynamicMaterialInstance _output_get 0 "/Game/Materials/Outline/m_outline_Inst.m_outline_Inst" "None" :!class /Script/Engine.PrimitiveComponent))
    (Rendering|Material|SetVectorParameterValue _returnvalue_2 "color" "(R=0.901042,G=0.671726,B=0.110566,A=1.000000)" :!class /Script/Engine.MaterialInstanceDynamic)
    (Rendering|Material|SetScalarParameterValue _returnvalue_2 "Scale" 8.0 :!class /Script/Engine.MaterialInstanceDynamic)
    (Variables|Default|SetbThereIsOutline true)))

(event Custom|ProgressBar
  (bind _returnvalue (Game|Player|GetPlayerPawn 0))
  (bind _returnvalue_2 (Game|Player|GetPlayerPawn 0))
  (bind _asthird_person_character (Utilities|Casting|CastToThirdPersonCharacter _returnvalue_2))
  (bind _asthird_person_character_2 (Utilities|Casting|CastToThirdPersonCharacter _returnvalue))
  (bind _mainhud (Variables|/Game/Blueprints/Core/ThirdPersonCharacter.ThirdPersonCharacter_C|GetMainHUD _asthird_person_character))
  ;[0.5469 0 1] Progress Bar
  (bind _avaibleinventoryslots (CallFunction|GetAvailableInventorySlots))
  (if (not (== _avaibleinventoryslots 0))
    (Default|StartExtracting _mainhud)
    (Utilities|FlowControl|Delay 4.0)
    (Variables|/Game/Blueprints/Core/ThirdPersonCharacter.ThirdPersonCharacter_C|SetbCanMove (.AsThird%20Person%20Character (Utilities|Casting|CastToThirdPersonCharacter (Game|Player|GetPlayerPawn 0))) true)
    (bind _successful (CallFunction|AddItemtoInventory (Variables|Default|GetExtractableItemInfo)))
    (if _successful
      (Default|ItemPickedUp (Variables|/Game/Blueprints/Core/ThirdPersonCharacter.ThirdPersonCharacter_C|GetMainHUD (.AsThird%20Person%20Character (Utilities|Casting|CastToThirdPersonCharacter (Game|Player|GetPlayerPawn 0)))) (Variables|Default|GetExtractableItemInfo))
      (bind _result (Math|Integer|DecrementInt (Variables|Default|GetExtractionTimesLeft))
        (:%20%20
          (if (== _result 0)
            (Variables|Default|SetExtractionPointState "NewEnumerator2")
            (Default|ShowExtactNotText _mainhud)
            (Utilities|FlowControl|Delay 1.2e+02)
            (Variables|Default|SetExtractionPointState "NewEnumerator0")
            (else
              (Variables|Default|SetExtractionPointState "NewEnumerator0")))))
      (else
        (Variables|Default|SetExtractionPointState "NewEnumerator0")))
    (else
      (Variables|/Game/Blueprints/Core/ThirdPersonCharacter.ThirdPersonCharacter_C|SetbCanMove _asthird_person_character_2 true)
      (Default|InventoryFull (Variables|/Game/Blueprints/Core/ThirdPersonCharacter.ThirdPersonCharacter_C|GetMainHUD _asthird_person_character_2))
      (Variables|Default|SetExtractionPointState "NewEnumerator0"))))

(event Custom|DeleteOutline
  (bind _outlinermesh (Variables|Default|GetOutlinerMesh))
  ;[1 0.4922 0] OutLine
  (Utilities|IsValid _outlinermesh
    (:Is%20Valid
      (Components|DestroyComponent _outlinermesh)
      (Variables|Default|SetbThereIsOutline false))))

(event EventBeginPlay
  (bind _extractableitemdatatable (Variables|Default|GetExtractableItemDataTable))
  (bind (_datatable _rowname) (Utilities|Struct|BreakDataTableRowHandle _extractableitemdatatable))
  ;[0.1615 0.3514 1] Begin Play
  (if (Variables|Default|GetbEnabled)
    (bind _returnvalue (Utilities|GetDataTableRow _datatable _rowname)
      (:then
        (Variables|Default|SetExtractableItemInfo _returnvalue)))))

(event EventStartInteraction
  (params (InteractiveActor :type Actor%20Object%20Reference))
  (bind _asthird_person_character (Utilities|Casting|CastToThirdPersonCharacter InteractiveActor))
  ;[1 0 0] Event Start Interaction
  (if (Variables|Default|GetbEnabled)
    (if (Utilities|Enum|Equal(Enum) (Variables|Default|GetExtractionPointState) "NewEnumerator0")
      (Variables|/Game/Blueprints/Core/ThirdPersonCharacter.ThirdPersonCharacter_C|SetbCanMove _asthird_person_character false)
      (Variables|Default|SetExtractionPointState "NewEnumerator1")
      (CallFunction|ProgressBar))
    (elif (Utilities|Enum|Equal(Enum) (Variables|Default|GetExtractionPointState) "NewEnumerator2")
      (Default|ShowExtactNotText (Variables|/Game/Blueprints/Core/ThirdPersonCharacter.ThirdPersonCharacter_C|GetMainHUD _asthird_person_character)))))

(fn ConstructionScript
  (Components|StaticMesh|SetStaticMesh (Variables|Default|GetMesh) (Variables|Default|GetStaticMesh))
  (Components|Capsule|SetCapsuleSize (Variables|Default|GetCapsule) (Variables|Default|GetCapsuleCollisionRadius) (Variables|Default|GetCapsuleHeight) true))