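; BP_Buzhon is a test mailbox actor that opens a quest list UI when the player interacts with it.
; Its box overlap registers it as the ThirdPersonCharacter's interactable and clears that on exit.
; StartInteraction disables character input, creates or reuses W_MailboxTest, switches to UI-only input with cursor and refreshes quests.
; The widget's close event collapses it and restores game input.
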(event OnComponentBeginOverlap(Box)
  (params (OverlappedComponent :type Primitive%20Component%20Object%20Reference) (OtherActor :type Actor%20Object%20Reference) (OtherComp :type Primitive%20Component%20Object%20Reference) (OtherBodyIndex :type Integer) (bFromSweep :type Boolean) (SweepResult :type Hit%20Result%20Structure%20%28by%20ref%29))
  ;[1 0.3281 0] Collision Box
  (bind _asthird_person_character (Utilities|Casting|CastToThirdPersonCharacter OtherActor))
  (Default|RegisterInteractableActor _asthird_person_character self))

(event OnComponentEndOverlap(Box)
  (params (OverlappedComponent :type Primitive%20Component%20Object%20Reference) (OtherActor :type Actor%20Object%20Reference) (OtherComp :type Primitive%20Component%20Object%20Reference) (OtherBodyIndex :type Integer))
  ;[1 0.3281 0] Collision Box
  (bind _asthird_person_character (Utilities|Casting|CastToThirdPersonCharacter OtherActor))
  (Default|RegisterInteractableActor _asthird_person_character))

(event Custom|CloseWidget
  (bind _returnvalue (Game|GetPlayerController 0))
  ;[0 1 0.7656] Close Widget
  (Widget|SetVisibility (Variables|Default|GetMailboxWidget) "Collapsed")
  (Variables|/Script/Engine.PlayerController|SetbShowMouseCursor _returnvalue false)
  (Input|SetInputModeGameOnly _returnvalue)
  (Input|EnableInput (.AsThird%20Person%20Character (Utilities|Casting|CastToThirdPersonCharacter (Game|Player|GetPlayerPawn 0))) _returnvalue))

(event EventBeginPlay)

(event Collision|EventActorBeginOverlap
  (params (OtherActor :type Actor%20Object%20Reference)))

(event EventTick
  (params (DeltaSeconds :type Float%20%28single-precision%29)))

(event EventStartInteraction
  (params (InteractiveActor :type Actor%20Object%20Reference))
  (bind _returnvalue (Game|GetPlayerController 0))
  (Input|DisableInput (.AsThird%20Person%20Character (Utilities|Casting|CastToThirdPersonCharacter InteractiveActor)) (Game|GetPlayerController 0))
  (Utilities|IsValid (Variables|Default|GetMailboxWidget)
    (:Is%20Valid
      (Widget|SetVisibility (Variables|Default|GetMailboxWidget) "Visible"))
    (:Is%20Not%20Valid
      (bind _returnvalue_2 (UserInterface|CreateWidget "/Game/Test/QuestsTest/W_MailboxTest.W_MailboxTest_C"))
      (bind _output_get (Variables|Default|SetMailboxWidget _returnvalue_2))
      (UserInterface|Viewport|AddtoViewport _output_get 0)
      (EventDispatchers|BindEventtoCloseClicked _output_get (delegate Custom|CloseWidget))
      ;[1 0.7266 0] Aquí van los binds
      (Development|PrintString "Hello")))
  (Variables|/Script/Engine.PlayerController|SetbShowMouseCursor _returnvalue true)
  (Input|SetInputModeUIOnly _returnvalue (Variables|Default|GetMailboxWidget) "LockInFullscreen")
  (Default|RefreshQuestList (Variables|Default|GetMailboxWidget)))

(fn ConstructionScript)