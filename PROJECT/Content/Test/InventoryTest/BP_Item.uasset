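; BP_Item is a pickup actor for an inventory test, configured from a data table row that sets its info and "Pick Up" label.
; Its box overlap toggles the label and registers or clears the item as the ThirdPersonCharacter's interactable.
; StartInteraction adds the actor itself to the GameInstance inventory up to a fixed cap, without destroying or hiding it.
; When the inventory is full, the label switches to a Spanish refusal message.
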(event OnComponentBeginOverlap(Box)
  (params (OverlappedComponent :type Primitive%20Component%20Object%20Reference) (OtherActor :type Actor%20Object%20Reference) (OtherComp :type Primitive%20Component%20Object%20Reference) (OtherBodyIndex :type Integer) (bFromSweep :type Boolean) (SweepResult :type Hit%20Result%20Structure%20%28by%20ref%29))
  (bind _asthird_person_character (Utilities|Casting|CastToThirdPersonCharacter OtherActor))
  (Rendering|SetVisibility (Variables|Default|GetTextRender) true false)
  (Default|RegisterInteractableActor _asthird_person_character self))

(event OnComponentEndOverlap(Box)
  (params (OverlappedComponent :type Primitive%20Component%20Object%20Reference) (OtherActor :type Actor%20Object%20Reference) (OtherComp :type Primitive%20Component%20Object%20Reference) (OtherBodyIndex :type Integer))
  (bind _asthird_person_character (Utilities|Casting|CastToThirdPersonCharacter OtherActor))
  (Rendering|SetVisibility (Variables|Default|GetTextRender) false false)
  (Default|RegisterInteractableActor _asthird_person_character))

(event EventBeginPlay)

(event Collision|EventActorBeginOverlap
  (params (OtherActor :type Actor%20Object%20Reference)))

(event EventTick
  (params (DeltaSeconds :type Float%20%28single-precision%29)))

(event EventStartInteraction
  (params (InteractiveActor :type Actor%20Object%20Reference))
  (bind _returnvalue (Game|GetGameInstance))
  (bind _asgi_main_game_instance (Utilities|Casting|CastToGI_MainGameInstance _returnvalue))
  (bind _inventory (Variables|/Game/Blueprints/Core/GI_MainGameInstance.GI_MainGameInstance_C|GetInventory _asgi_main_game_instance))
  (if (< (Utilities|Array|Length _inventory) 10)
    (Utilities|Array|Add _inventory self)
    (else
      (Rendering|Components|TextRender|SetText (Variables|Default|GetTextRender) (Utilities|Text|FormatText "No puedes recogerme")))))

(fn ConstructionScript
  (bind _item (Variables|Default|Getitem))
  (bind (_datatable _rowname) (Utilities|Struct|BreakDataTableRowHandle _item))
  (bind _returnvalue (Utilities|GetDataTableRow _datatable _rowname)
    (:then
      (Variables|Default|SetitemInfo _returnvalue)
      (Rendering|Components|TextRender|SetText (Variables|Default|GetTextRender) (Utilities|Text|ToText(String) (Utilities|String|Append "Pick Up (" (.Nombre (Utilities|Struct|BreakST_ItemStruct _returnvalue)) ")"))))))