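; Interactable cauldron actor where the player crafts potions through UI and collects the result into the Game Instance inventory.
; Its collision box registers it with the character and shows a camera-facing prompt when idle.
; A state enum selects the crafting or collection widget, whose dispatchers call back into the cauldron.
; Crafting spawns the recipe's DataTable item, or PlumaFenix on failure, and starts a progress-bar timeline meant to mark it ready.
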(event OnComponentBeginOverlap(Box)
  (params (OverlappedComponent :type Primitive%20Component%20Object%20Reference) (OtherActor :type Actor%20Object%20Reference) (OtherComp :type Primitive%20Component%20Object%20Reference) (OtherBodyIndex :type Integer) (bFromSweep :type Boolean) (SweepResult :type Hit%20Result%20Structure%20%28by%20ref%29))
  (bind _returnvalue (Game|GetPlayerCameraManager 0))
  ;[0 0.7422 1] Collision Box
  (bind _asthird_person_character (Utilities|Casting|CastToThirdPersonCharacter OtherActor))
  (Rendering|SetVisibility (Variables|Default|GetTextRender) (Utilities|Enum|Equal(Enum) (Variables|Default|GetCauldronState) "NewEnumerator0") false)
  (Default|RegisterInteractableActor _asthird_person_character self)
  (Utilities|IsValid _returnvalue
    (:Is%20Valid
      (Transformation|SetWorldRotation (Variables|Default|GetTextRender) (Math|Rotator|FindLookatRotation (Transformation|GetWorldLocation (Variables|Default|GetTextRender)) (Camera|GetCameraLocation _returnvalue)) false false))))

(event OnComponentEndOverlap(Box)
  (params (OverlappedComponent :type Primitive%20Component%20Object%20Reference) (OtherActor :type Actor%20Object%20Reference) (OtherComp :type Primitive%20Component%20Object%20Reference) (OtherBodyIndex :type Integer))
  ;[0 0.7422 1] Collision Box
  (bind _asthird_person_character (Utilities|Casting|CastToThirdPersonCharacter OtherActor))
  (Rendering|SetVisibility (Variables|Default|GetTextRender) false true)
  (Default|RegisterInteractableActor _asthird_person_character))

(event Custom|MakingPotion
  (params (Successful :type Boolean) (Recipe :type ST%20Recipes%20Struct%20Structure))
  (Variables|Default|SetCauldronState "NewEnumerator1")
  (CallFunction|CloseCraftWidget)
  (Rendering|SetVisibility (Variables|Default|GetTextRender) false true)
  (Rendering|SetVisibility (Variables|Default|GetWidget) true true)
  (Components|Timeline|PlayfromStart (Variables|Default|GetTL_ProgressBar))
  (if Successful
    (bind _outrownames (DataTable|GetDataTableRowNames "/Game/Test/InventoryTest/Lista_de_ítems_-_Hoja_1.Lista_de_ítems_-_Hoja_1"))
    (bind _array_element (Utilities|Array|ForEachLoopwithBreak _outrownames :!label _label)
      (:LoopBody
        (bind _returnvalue (Utilities|GetDataTableRow "/Game/Test/InventoryTest/Lista_de_ítems_-_Hoja_1.Lista_de_ítems_-_Hoja_1" _array_element)
          (:then
            (if (Utilities|Enum|Equal(Enum) (.Nombre (Utilities|Struct|BreakST_ItemStruct _returnvalue)) (.Nombre (Utilities|Struct|BreakST_RecipesStruct Recipe)))
              (bind _returnvalue_2 (Game|SpawnActorfromClass "/Game/Test/InventoryTest/BP_Item.BP_Item_C" (Math|Transform|MakeTransform "0, 0, 0" "0, 0, 0" "1,1,1") "AlwaysSpawn" 0 _returnvalue 0))
              (Variables|Default|SetCreatedItem _returnvalue_2)
              (goto _label Break))))))
    (else
      (bind _returnvalue_3 (Utilities|GetDataTableRow "/Game/Test/InventoryTest/Lista_de_ítems_-_Hoja_1.Lista_de_ítems_-_Hoja_1" "PlumaFenix")
        (:then
          (bind _returnvalue_4 (Game|SpawnActorfromClass "/Game/Test/InventoryTest/BP_Item.BP_Item_C" (Math|Transform|MakeTransform "0, 0, 0" "0, 0, 0" "1,1,1") "AlwaysSpawn" 0 _returnvalue_3 0))
          (Variables|Default|SetCreatedItem _returnvalue_4))))))

(event Custom|CloseTab
  (Widget|SetVisibility (Variables|Default|GetPopUpWidget) "Collapsed")
  (Utilities|Array|Add (Variables|/Game/Blueprints/Core/GI_MainGameInstance.GI_MainGameInstance_C|GetInventory (.AsGI%20Main%20Game%20Instance (Utilities|Casting|CastToGI_MainGameInstance (Game|GetGameInstance)))) (Variables|Default|GetCreatedItem)))

(event Custom|CloseCraftWidget
  (bind _returnvalue (Game|GetPlayerController 0))
  (Widget|SetVisibility (Variables|Default|GetCraftWidget) "Collapsed")
  (Input|SetInputModeGameOnly _returnvalue)
  (Input|EnableInput _returnvalue _returnvalue))

(event Collision|EventActorBeginOverlap
  (params (OtherActor :type Actor%20Object%20Reference)))

(event EventStartInteraction
  (params (InteractiveActor :type Actor%20Object%20Reference))
  (bind _returnvalue (Game|GetPlayerController 0))
  (bind _returnvalue_2 (Game|GetPlayerController 0))
  (bind _cauldronstate (Variables|Default|GetCauldronState))
  (if (Utilities|Enum|NotEqual(Enum) _cauldronstate "NewEnumerator1")
    (if (Utilities|Enum|Equal(Enum) _cauldronstate "NewEnumerator0")
      (Input|DisableInput (.AsThird%20Person%20Character (Utilities|Casting|CastToThirdPersonCharacter InteractiveActor)) (Game|GetPlayerController 0))
      (Utilities|IsValid (Variables|Default|GetCraftWidget)
        (:Is%20Valid
          (Widget|SetVisibility (Variables|Default|GetCraftWidget) "Visible"))
        (:Is%20Not%20Valid
          (bind _returnvalue_3 (UserInterface|CreateWidget "/Game/Test/CratingTest/W_CraftingInterface.W_CraftingInterface_C"))
          (bind _output_get (Variables|Default|SetCraftWidget _returnvalue_3))
          (UserInterface|Viewport|AddtoViewport _output_get 0)
          (EventDispatchers|BindEventtoWidgetClosed _output_get (delegate Custom|CloseCraftWidget))
          (EventDispatchers|BindEventtoMadeCombination _output_get (delegate Custom|MakingPotion))))
      (Variables|/Script/Engine.PlayerController|SetbShowMouseCursor _returnvalue_2 true)
      (Input|SetInputModeGameandUI _returnvalue_2 0 "LockInFullscreen" true)
      (Default|RefreshComboBoxes _output_get)
      (else
        (Input|DisableInput (.AsThird%20Person%20Character (Utilities|Casting|CastToThirdPersonCharacter InteractiveActor)) (Game|GetPlayerController 0))
        (Utilities|IsValid (Variables|Default|GetPopUpWidget)
          (:Is%20Valid
            (Widget|SetVisibility (Variables|Default|GetPopUpWidget) "Visible"))
          (:Is%20Not%20Valid
            (bind _returnvalue_4 (UserInterface|CreateWidget "/Game/Test/CratingTest/W_CollectPotion.W_CollectPotion_C"))
            (bind _output_get_2 (Variables|Default|SetPopUpWidget _returnvalue_4))
            (UserInterface|Viewport|AddtoViewport _output_get_2 0)
            (EventDispatchers|BindEventtoCloseTab _returnvalue_4 (delegate Custom|CloseTab))))
        (Variables|/Script/Engine.PlayerController|SetbShowMouseCursor _returnvalue true)
        (Input|SetInputModeGameandUI _returnvalue 0 "LockInFullscreen" true)
        (Default|RefreshItem (Variables|Default|GetPopUpWidget) (Variables|/Game/Test/InventoryTest/BP_Item.BP_Item_C|GetitemInfo (Variables|Default|GetCreatedItem)))))))

(fn ConstructionScript)