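; Foliage-folder spline Blueprint that lays a chosen static mesh along its spline as a chain of deformed spline mesh segments.
; The construction script adds one segment per spacing interval plus a final remainder segment with proportionally shortened tangents.
; Each segment takes offset end positions, tangents and scale from the spline.
; The midpoint supplies the up vector, and start and end roll are measured relative to its rotation so segments follow spline twist.
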(event EventBeginPlay)

(event Collision|EventActorBeginOverlap
  (params (OtherActor :type Actor%20Object%20Reference)))

(event EventTick
  (params (DeltaSeconds :type Float%20%28single-precision%29)))

(fn ConstructionScript
  (bind _spacing (Variables|Default|GetSpacing))
  (bind _spline (Variables|Default|GetSpline))
  (bind _returnvalue (Spline|GetSplineLength _spline))
  (bind (_remainder _returnvalue_2) (Math|Float|Division(WholeandRemainder) _returnvalue _spacing))
  (for _index (range 0 _returnvalue_2)
    (bind _output_get (Variables|Default|SetIndex _index))
    (Variables|Default|SetFinal%20Tangent%20Scale (select (== _output_get _returnvalue_2) (* (/ _remainder (Variables|Default|GetSpacing)) (Variables|Default|GetTangent%20Scale)) (Variables|Default|GetTangent%20Scale)))
    (bind _output_get_2 (Variables|Default|SetStart%20Distance (* (Variables|Default|GetIndex) (Variables|Default|GetSpacing))))
    (Variables|Default|SetMiddle%20Distance (+ _output_get_2 (* (Variables|Default|GetSpacing) 0.5)))
    (Variables|Default|SetEnd%20Distance (+ (Variables|Default|GetStart%20Distance) (Variables|Default|GetSpacing)))
    (bind _returnvalue_3 (AddComponent|AddSplineMeshComponent false))
    (bind _output_get_3 (Variables|Default|SetSpline%20Mesh _returnvalue_3))
    (SplineMesh|SetStartandEnd _output_get_3 (Spline|GetLocationatDistanceAlongSpline (Variables|Default|GetSpline) (- (Variables|Default|GetStart%20Distance) (Variables|Default|GetStart%20Offset)) "Local") (* (Spline|GetDirectionatDistanceAlongSpline (Variables|Default|GetSpline) (Variables|Default|GetStart%20Distance) "Local") (Variables|Default|GetFinal%20Tangent%20Scale)) (Spline|GetLocationatDistanceAlongSpline (Variables|Default|GetSpline) (+ (Variables|Default|GetEnd%20Distance) (Variables|Default|GetEnd%20Offset)) "Local") (* (Spline|GetDirectionatDistanceAlongSpline (Variables|Default|GetSpline) (Variables|Default|GetEnd%20Distance) "Local") (Variables|Default|GetFinal%20Tangent%20Scale)) true :!class /Script/Engine.SplineMeshComponent)
    (SplineMesh|SetStartScale (Variables|Default|GetSpline%20Mesh) (Math|Vector2D|MakeVector2D (.Y (Math|Vector|BreakVector (Class|SplineComponent|GetScaleatDistanceAlongSpline (Variables|Default|GetSpline) (Variables|Default|GetStart%20Distance)))) (.Z (Math|Vector|BreakVector (Class|SplineComponent|GetScaleatDistanceAlongSpline (Variables|Default|GetSpline) (Variables|Default|GetStart%20Distance))))) true :!class /Script/Engine.SplineMeshComponent)
    (SplineMesh|SetEndScale (Variables|Default|GetSpline%20Mesh) (Math|Vector2D|MakeVector2D (.Y (Math|Vector|BreakVector (Class|SplineComponent|GetScaleatDistanceAlongSpline (Variables|Default|GetSpline) (Variables|Default|GetEnd%20Distance)))) (.Z (Math|Vector|BreakVector (Class|SplineComponent|GetScaleatDistanceAlongSpline (Variables|Default|GetSpline) (Variables|Default|GetEnd%20Distance))))) true :!class /Script/Engine.SplineMeshComponent)
    (SplineMesh|SetSplineUpDir (Variables|Default|GetSpline%20Mesh) (Class|SplineComponent|GetUpVectoratDistanceAlongSpline (Variables|Default|GetSpline) (Variables|Default|GetMiddle%20Distance) "World") true)
    (Class|SplineMeshComponent|SetStartRoll (Variables|Default|GetSpline%20Mesh) (Math|Trig|DegreesToRadians (.Roll (Math|Rotator|BreakRotator (Math|Rotator|CombineRotators (Spline|GetRotationatDistanceAlongSpline (Variables|Default|GetSpline) (Variables|Default|GetStart%20Distance) "Local") (Class|KismetMathLibrary|NegateRotator (Spline|GetRotationatDistanceAlongSpline (Variables|Default|GetSpline) (Variables|Default|GetMiddle%20Distance) "Local")))))) true)
    (Class|SplineMeshComponent|SetEndRoll (Variables|Default|GetSpline%20Mesh) (Math|Trig|DegreesToRadians (.Roll (Math|Rotator|BreakRotator (Math|Rotator|CombineRotators (Spline|GetRotationatDistanceAlongSpline (Variables|Default|GetSpline) (Variables|Default|GetEnd%20Distance) "Local") (Class|KismetMathLibrary|NegateRotator (Spline|GetRotationatDistanceAlongSpline (Variables|Default|GetSpline) (Variables|Default|GetMiddle%20Distance) "Local")))))) true)
    (Components|StaticMesh|SetStaticMesh (Variables|Default|GetSpline%20Mesh) (Variables|Default|GetMesh))))