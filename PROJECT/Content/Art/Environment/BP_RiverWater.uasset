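; BP_RiverWater is a spline-based river water actor that builds its surface along an editable spline.
; Its construction script adds one spline mesh component per segment between consecutive points and applies the Material variable to each.
; Each segment takes its start and end positions and tangents from the spline in local space.
; Per-point spline scale, multiplied by EasyScale, sets each end's cross-section, so the river can vary along its length.
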(fn ConstructionScript
  (bind _spline (Variables|Default|GetSpline))
  (bind _easyscale (Variables|Variables|GetEasyScale))
  (bind _easyscale_2 (Variables|Variables|GetEasyScale))
  ;[1 1 1] Loop through spline points
  (for _index (range 0 (- (Spline|GetNumberOfSplinePoints (Variables|Default|GetSpline)) 2))
    (bind _returnvalue (AddComponent|AddSplineMeshComponent false))
    (Rendering|Material|SetMaterial _returnvalue 0 (Variables|Variables|GetMaterial))
    (SplineMesh|SetStartScale _returnvalue (Math|Vector2D|MakeVector2D (* (.x (Spline|GetScaleatSplinePoint (Variables|Default|GetSpline) _index)) _easyscale) (* _easyscale (.y (Spline|GetScaleatSplinePoint (Variables|Default|GetSpline) _index)))) true :!class /Script/Engine.SplineMeshComponent)
    (SplineMesh|SetEndScale _returnvalue (Math|Vector2D|MakeVector2D (* (.x (Spline|GetScaleatSplinePoint (Variables|Default|GetSpline) (+ _index 1))) _easyscale_2) (* _easyscale_2 (.y (Spline|GetScaleatSplinePoint (Variables|Default|GetSpline) (+ _index 1))))) true :!class /Script/Engine.SplineMeshComponent)
    (SplineMesh|SetStartandEnd _returnvalue (.Location (Spline|GetLocationandTangentatSplinePoint _spline _index "Local")) (.Tangent (Spline|GetLocationandTangentatSplinePoint _spline _index "Local")) (.Location (Spline|GetLocationandTangentatSplinePoint _spline (+ _index 1) "Local")) (.Tangent (Spline|GetLocationandTangentatSplinePoint _spline (+ _index 1) "Local")) true :!class /Script/Engine.SplineMeshComponent)))