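; Outline actor Blueprint that displays a configurable static mesh and can add or remove an outline on demand.
; On BeginPlay it assigns Mesh to its StaticMesh component.
; createoutline spawns one duplicate mesh component and sets color and Scale on a dynamic instance of its slot 0 material.
; deleteoutline destroys that component and clears the HasOutline guard so the outline can be recreated.
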(event Custom|create%20outline
  (if (not (Variables|Default|Gethas%20outline))
    (bind _returnvalue (AddComponent|AddStaticMeshComponent false (Transformation|GetWorldTransform (Variables|Default|GetStaticMesh))))
    (bind _output_get (Variables|Default|SetMesh%20Component _returnvalue))
    (Components|StaticMesh|SetStaticMesh _output_get (Variables|Default|Getmesh))
    (bind _returnvalue_2 (Rendering|Material|CreateDynamicMaterialInstance _output_get 0 0 "None" :!class /Script/Engine.PrimitiveComponent))
    (Rendering|Material|SetVectorParameterValue _returnvalue_2 "color" (Variables|Default|Getcolor) :!class /Script/Engine.MaterialInstanceDynamic)
    (Rendering|Material|SetScalarParameterValue _returnvalue_2 "Scale" (Variables|Default|Getscale) :!class /Script/Engine.MaterialInstanceDynamic)
    (Variables|Default|Sethas%20outline true)))

(event Custom|delete%20outline
  (bind _mesh_component (Variables|Default|GetMesh%20Component))
  (Utilities|IsValid _mesh_component
    (:Is%20Valid
      (Components|DestroyComponent _mesh_component)
      (Variables|Default|Sethas%20outline false))))

(event EventBeginPlay
  (Components|StaticMesh|SetStaticMesh (Variables|Default|GetStaticMesh) (Variables|Default|Getmesh)))

(event Collision|EventActorBeginOverlap
  (params (OtherActor :type Actor%20Object%20Reference)))

(event EventTick
  (params (DeltaSeconds :type Float%20%28single-precision%29)))

(fn ConstructionScript)