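; Motion-controller blade actor that slices procedural meshes it swings through.
; Each tick it derives velocity from a tracker socket and allows slicing only for fast, edge-aligned swings (optionally double-edged), switching collision between overlap and block accordingly.
; A qualifying overlap, briefly debounced, cuts the mesh along the blade's plane with a capped face.
; The new half becomes a physics body with copied damping and gravity enabled.
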(event OnComponentBeginOverlap(Blade_StaticMesh)
  (params (OverlappedComponent :type Primitive%20Component%20Object%20Reference) (OtherActor :type Actor%20Object%20Reference) (OtherComp :type Primitive%20Component%20Object%20Reference) (OtherBodyIndex :type Integer) (bFromSweep :type Boolean) (SweepResult :type Hit%20Result%20Structure%20%28by%20ref%29))
  ;[0 0.22 0.07084] Begin Overlap
  (if (Variables|Default|GetCan%20Slice%20Objects)
    (bind _asprocedural_mesh_component (Utilities|Casting|CastToProceduralMeshComponent OtherComp))
    (Utilities|FlowControl|DoOnce false :!label _label
      (:Completed
        (CallFunction|PerformProcMeshSlicing _asprocedural_mesh_component)
        (Utilities|FlowControl|Delay 0.08)
        (goto _label Reset)))))

(event Custom|Setup%20Controller
  (params (In%20Parent :type Scene%20Component%20Object%20Reference) (Hand :type EControllerHand%20Enum :default "Left"))
  ;[0.075 0 0] Custom Events
  (Transformation|AttachComponentToComponent (Variables|Default|GetMotionController) In%20Parent "None" "SnapToTarget" "SnapToTarget" "KeepRelative" true)
  (Variables|/Script/HeadMountedDisplay.MotionControllerComponent|SetHand (Variables|Default|GetMotionController) Hand))

(event EventTick
  (params (DeltaSeconds :type Float%20%28single-precision%29))
  (bind _blade_staticmesh (Variables|Default|GetBlade_StaticMesh))
  (bind _returnvalue (Transformation|GetSocketLocation _blade_staticmesh "PositionTracker"))
  ;[0 0.04993 0.19] Tick
  (Variables|Default|SetDelta%20Seconds DeltaSeconds)
  (Utilities|FlowControl|Sequence
    (:then_0
      (Variables|Default|SetTracker%20Velocity (/ (- _returnvalue (Variables|Default|GetLast%20Frame%20Tracker%20Position)) (Variables|Default|GetDelta%20Seconds)))
      (Variables|Default|SetLast%20Frame%20Tracker%20Position _returnvalue)
      (Variables|Default|SetCan%20Slice%20Objects (and (> (select (Variables|Default|GetIs%20Double%20Edged) (Math|Float|Absolute(Float) (Math|Vector|DotProduct (Math|Vector|Normalize (Variables|Default|GetTracker%20Velocity)) (Math|Vector|GetRightVector (Variables|Default|GetBlade_StaticMesh)))) (Math|Vector|DotProduct (Math|Vector|Normalize (Variables|Default|GetTracker%20Velocity)) (Math|Vector|GetRightVector (Variables|Default|GetBlade_StaticMesh)))) 0.9) (> (Math|Vector|VectorLength (Variables|Default|GetTracker%20Velocity)) (Variables|Default|GetMin%20Velocity%20To%20Perform%20Slicing)))))
    (:then_1
      (Collision|SetCollisionProfileName (Variables|Default|GetBlade_StaticMesh) (select (Variables|Default|GetCan%20Slice%20Objects) "OverlapAll" "BlockAll") true :!class /Script/Engine.PrimitiveComponent))))

(fn ConstructionScript)

(fn PerformProcMeshSlicing
  (params (In%20Procedural%20Mesh :type Procedural%20Mesh%20Component%20Object%20Reference))
  (LocalVariables|SetIn%20ProcMesh In%20Procedural%20Mesh)
  (bind _outotherhalfprocmesh (Class|KismetProceduralMeshLibrary|SliceProceduralMesh (LocalVariables|GetIn%20ProcMesh) (.OutPointOnBody (Collision|GetClosestPointonCollision (LocalVariables|GetIn%20ProcMesh) (Transformation|GetWorldLocation (Variables|Default|GetBlade_StaticMesh)) "None")) (Math|Vector|GetForwardVector (Variables|Default|GetBlade_StaticMesh)) true "CreateNewSectionForCap" "/Game/ObjectSlicing/Assets/Materials/M_ShapeCap.M_ShapeCap"))
  (bind _output_get (LocalVariables|SetOut%20Half%20ProcMesh _outotherhalfprocmesh))
  (Transformation|AttachComponentToComponent _output_get (Transformation|GetAttachParent (LocalVariables|GetIn%20ProcMesh)) "None" "KeepWorld" "KeepWorld" "KeepWorld" true)
  (Class|PrimitiveComponent|SetLinearDamping (LocalVariables|GetOut%20Half%20ProcMesh) (Class|PrimitiveComponent|GetLinearDamping (LocalVariables|GetIn%20ProcMesh)))
  (Class|PrimitiveComponent|SetAngularDamping (LocalVariables|GetOut%20Half%20ProcMesh) (Class|PrimitiveComponent|GetAngularDamping (LocalVariables|GetIn%20ProcMesh)))
  (Physics|SetSimulatePhysics (LocalVariables|GetOut%20Half%20ProcMesh) true)
  (Physics|SetEnableGravity (LocalVariables|GetOut%20Half%20ProcMesh) true)
  (return (LocalVariables|GetOut%20Half%20ProcMesh)))